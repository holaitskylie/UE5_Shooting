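; Kh-31P missile actor that flies straight ahead and destroys any BP_Enemy it overlaps, spawning an explosion, adding score through BP_GameModeBase and destroying itself.
; Tick moves it along its forward vector at MoveSpeed without sweeping.
; BeginPlay caches its anim instance, which four fin events feed with normalized inputs remapped to clamped deflection angles.
; A separate event toggles the thruster effect.
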(event Custom|SetEngineState
  (params (bEngineActive :type Boolean))
  ;[1 1 1] Set engine state
  (Components|Activation|SetActive (Variables|Default|GetThrusterFX) bEngineActive true))

(event Custom|SetFin1Angle
  (params (Angle :type Float%20%28double-precision%29))
  (Variables|/Game/Modelings/VigilanteContent/Projectiles/East_Missile_Kh31P/ABP_East_Missile_Kh31P.ABP_East_Missile_Kh31P_C|SetFin1Angle (Variables|Default|GetAnimInstance) (Math|Float|MapRangeClamped Angle -1.0 1.0 -45.0 45.0)))

(event Custom|SetFin2Angle
  (params (Angle :type Float%20%28double-precision%29))
  (Variables|/Game/Modelings/VigilanteContent/Projectiles/East_Missile_Kh31P/ABP_East_Missile_Kh31P.ABP_East_Missile_Kh31P_C|SetFin2Angle (Variables|Default|GetAnimInstance) (Math|Float|MapRangeClamped Angle -1.0 1.0 -45.0 45.0)))

(event Custom|SetFin3Angle
  (params (Angle :type Float%20%28double-precision%29))
  (Variables|/Game/Modelings/VigilanteContent/Projectiles/East_Missile_Kh31P/ABP_East_Missile_Kh31P.ABP_East_Missile_Kh31P_C|SetFin3Angle (Variables|Default|GetAnimInstance) (Math|Float|MapRangeClamped Angle -1.0 1.0 -45.0 45.0)))

(event Custom|SetFin4Angle
  (params (Angle :type Float%20%28double-precision%29))
  (Variables|/Game/Modelings/VigilanteContent/Projectiles/East_Missile_Kh31P/ABP_East_Missile_Kh31P.ABP_East_Missile_Kh31P_C|SetFin4Angle (Variables|Default|GetAnimInstance) (Math|Float|MapRangeClamped Angle -1.0 1.0 -45.0 45.0)))

(event EventBeginPlay
  (bind _asabp_east_missile_kh_31p (Utilities|Casting|CastToABP_East_Missile_Kh31P (Components|SkeletalMesh|GetAnimInstance (Variables|Default|GetSkeletalMesh))))
  (Variables|Default|SetAnimInstance _asabp_east_missile_kh_31p))

(event Collision|EventActorBeginOverlap
  (params (OtherActor :type Actor%20Object%20Reference))
  (bind _asbp_enemy (Utilities|Casting|CastToBP_Enemy OtherActor))
  (Actor|DestroyActor _asbp_enemy)
  (Effects|SpawnEmitteratLocation "/Game/Realistic_Starter_VFX_Pack_Vol2/Particles/Explosion/P_Explosion_Big_A.P_Explosion_Big_A" (Transformation|GetActorLocation))
  (bind _asbp_game_mode_base (Utilities|Casting|CastToBP_GameModeBase (Game|GetGameMode)))
  (Default|AddScore _asbp_game_mode_base 1)
  (Actor|DestroyActor))

(event EventTick
  (params (DeltaSeconds :type Float%20%28single-precision%29))
  (Transformation|SetActorLocation (+ (Transformation|GetActorLocation) (* (* (Transformation|GetActorForwardVector) (Variables|Default|GetmoveSpeed)) DeltaSeconds)) false false))

(fn ConstructionScript)