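; BP_Bullet is a projectile actor that destroys enemies it touches.
; On Tick it moves along its forward vector at MoveSpeed, scaled by delta time, without sweeping.
; When it overlaps a BP_Enemy, it destroys that enemy, spawns a big explosion particle at its own location and destroys itself, ignoring other overlapping actors.
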(event EventBeginPlay)

(event Collision|EventActorBeginOverlap
  (params (OtherActor :type Actor%20Object%20Reference))
  (bind _asbp_enemy (Utilities|Casting|CastToBP_Enemy OtherActor))
  (Actor|DestroyActor _asbp_enemy)
  (Effects|SpawnEmitteratLocation "/Game/Realistic_Starter_VFX_Pack_Vol2/Particles/Explosion/P_Explosion_Big_B.P_Explosion_Big_B" (Transformation|GetActorLocation))
  (Actor|DestroyActor))

(event EventTick
  (params (DeltaSeconds :type Float%20%28single-precision%29))
  (Transformation|SetActorLocation (+ (Transformation|GetActorLocation) (* (* (Transformation|GetActorForwardVector) (Variables|Default|GetmoveSpeed)) DeltaSeconds)) false false))

(fn ConstructionScript)